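; BP_PickupBase4 is an interactable item pickup actor that hands its ItemData to the interacting player's inventory.
; SetItemData stores the data and applies its mesh and material.
; ExecuteInteraction calls TryPickupItem with the Alt-key state read from player 0's first-person character, then refreshes the interactor's hand visuals.
; It then destroys itself without checking whether the pickup succeeded.
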(event EventBeginPlay)

(event Collision|EventActorBeginOverlap
  (params (OtherActor :type Actor%20Object%20Reference)))

(event EventTick
  (params (DeltaSeconds :type Float%20%28single-precision%29)))

(event EventExecuteInteraction
  (params (InteractingPlayer :type Actor%20Object%20Reference))
  (bind _asbp_first_person_character (Utilities|Casting|CastToBP_FirstPersonCharacter (Game|GetPlayerCharacter 0)))
  (Class|InventoryComponent|TryPickupItem (Actor|GetComponentbyClass InteractingPlayer "/Script/FPSTest.InventoryComponent") (Variables|Default|GetItemData) (Variables|/Game/ThirdPerson/Blueprints/BP_FirstPersonCharacter.BP_FirstPersonCharacter_C|GetbIsAltDown _asbp_first_person_character))
  (bind _asbp_first_person_character_2 (Utilities|Casting|CastToBP_FirstPersonCharacter InteractingPlayer))
  (Default|RefreshHandVisuals _asbp_first_person_character_2)
  (Actor|DestroyActor))

(fn ConstructionScript)

(fn SetItemData
  (params (NewItemData :type Item%20Data%20Object%20Reference))
  (bind _staticmesh (Variables|Default|GetStaticMesh))
  (Variables|Default|SetItemData NewItemData)
  (Components|StaticMesh|SetStaticMesh _staticmesh (Variables|/Script/FPSTest.ItemData|GetPickupMesh NewItemData))
  (Rendering|Material|SetMaterial _staticmesh 0 (Variables|/Script/FPSTest.ItemData|GetItemMaterial NewItemData)))